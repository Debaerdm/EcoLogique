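; Interactive door actor that swings open or shut when E is pressed near it.
; The Inside trigger enables player input and opens a gate when a Client_BP enters, then disables input when it leaves.
; E passes through the gate to toggle Open and play or reverse the DoorSwing timeline.
; Each timeline update combines OpenAngle yaw with the door's rotation saved at BeginPlay, so the swing is relative to its placement.
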(event `self.ReceiveBeginPlay`
  (set `self.InitRotator` (`SceneComponent.K2_GetComponentRotation` (`self.Door`))))

(event `Key|E`
  (params (Key :type "Key Structure"))
  (:`Pressed`
    (`/Engine/EditorBlueprintResources/StandardMacros.Gate` true :!label _label
      (:`Exit`
        (if (`self.Open?`)
          (set `self.Open?` false)
          (bind (_direction _openangle) (`Timeline|DoorSwing` :!via `Reverse` :!label _label_2)
            (:`Update`
              (`SceneComponent.K2_SetWorldRotation` (`self.Door`) (`KismetMathLibrary.ComposeRotators` (`KismetMathLibrary.MakeRotator` 0.0 0.0 _openangle) (`self.InitRotator`)) false false)))
          (else
            (set `self.Open?` true)
            (goto _label_2)))))))

(event `self.Inside.OnComponentBeginOverlap`
  (params (OverlappedComponent :type "PrimitiveComponent Object Reference") (OtherActor :type "Actor Object Reference") (OtherComp :type "PrimitiveComponent Object Reference") (OtherBodyIndex :type Integer) (bFromSweep :type Boolean) (SweepResult :type "HitResult Structure (by ref)"))
  (cast `/Game/Client/Client_BP` OtherActor)
  (`self.EnableInput` (`GameplayStatics.GetPlayerController` 0))
  (goto _label :!via `Open`))

(event `self.Inside.OnComponentEndOverlap`
  (params (OverlappedComponent :type "PrimitiveComponent Object Reference") (OtherActor :type "Actor Object Reference") (OtherComp :type "PrimitiveComponent Object Reference") (OtherBodyIndex :type Integer))
  (cast `/Game/Client/Client_BP` OtherActor)
  (`self.DisableInput` (`GameplayStatics.GetPlayerController` 0)))

(fn `UserConstructionScript`)