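; Client_BP is a player-controlled Character that handles movement, camera look and jumping.
; Axis inputs move it along the camera's forward and right vectors or world up for SwimUp, and turn the view directly or through frame-time-scaled rates.
; The Jump action and first-finger touch share JumpEvent, which jumps and sets the Jump flag on the LutinAnim_Bp animation instance; landing clears it.
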(event `InputAxis|MoveForward`
  (params (AxisValue :type "Float (single-precision)"))
  ;[1 1 1] Mouvement
  (`self.AddMovementInput` (`SceneComponent.GetForwardVector` (`self.Camera`)) AxisValue))

(event `InputAxis|TurnRate`
  (params (AxisValue :type "Float (single-precision)"))
  ;[1 1 1] The gamepad controller for camera
  (`self.AddControllerYawInput` (* AxisValue (`GameplayStatics.GetWorldDeltaSeconds`) (`self.BaseTurnRate`))))

(event `InputAction|Jump`
  (params (Key :type "Key Structure"))
  ;[1 1 1] Sauter et tomber
  (:`Pressed`
    (`self.JumpEvent`)))

(event `InputAxis|MoveRight`
  (params (AxisValue :type "Float (single-precision)"))
  ;[1 1 1] Mouvement
  (`self.AddMovementInput` (`SceneComponent.GetRightVector` (`self.Camera`)) AxisValue))

(event `InputAxis|LookUpRate`
  (params (AxisValue :type "Float (single-precision)"))
  ;[1 1 1] The gamepad controller for camera
  (`self.AddControllerPitchInput` (* AxisValue (`GameplayStatics.GetWorldDeltaSeconds`) (`self.BaseLookUpRate`))))

(event `self.OnLanded`
  (params (Hit :type "HitResult Structure (by ref)"))
  ;[1 1 1] Sauter et tomber
  (bind _aslutin_anim_bp (cast `/Game/Client/LutinAnim_Bp` (`SkeletalMeshComponent.GetAnimInstance` (`self.Mesh`))))
  (set `/Game/Client/LutinAnim_Bp.Jump?` false _aslutin_anim_bp))

(event `InputTouch`
  (params (Location :type "Vector Structure") (FingerIndex :type "ETouchIndex Enum"))
  ;[1 1 1] Make jump
  (:`Pressed`
    (if (`|EnumEquality` FingerIndex "Touch1")
      (`self.JumpEvent`))))

(event `InputAxis|Turn`
  (params (AxisValue :type "Float (single-precision)"))
  ;[1 1 1] Rotation de la camera
  (`self.AddControllerYawInput` AxisValue))

(event `InputAxis|LookUp`
  (params (AxisValue :type "Float (single-precision)"))
  ;[1 1 1] Rotation de la camera
  (`self.AddControllerPitchInput` AxisValue))

(event `JumpEvent`
  ;[1 1 1] L'evenement pour sauter
  (`self.Jump`)
  (bind _aslutin_anim_bp (cast `/Game/Client/LutinAnim_Bp` (`SkeletalMeshComponent.GetAnimInstance` (`self.Mesh`))))
  (set `/Game/Client/LutinAnim_Bp.Jump?` true _aslutin_anim_bp))

(event `InputAxis|SwimUp`
  (params (AxisValue :type "Float (single-precision)"))
  (`self.AddMovementInput` (0.0 0.0 1.0) AxisValue))

(fn `UserConstructionScript`)